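; BP_TerrainGenerator is an actor that builds a square tile map of BP_Cube floor pieces enclosed by a BP_Boundaries ring.
; The SpawnMap event calls BuildMap, which destroys previously spawned pieces, then refills both tracking arrays.
; A nested loop sized from MapSize and TileGap centers the grid on the root, placing raised boundaries on the outer edge and cubes inside.
; Helper functions return the map's world size and its min/max coordinates.
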(event `self.ReceiveBeginPlay`)

(event `SpawnMap`
  (`self.BuildMap`))

(fn `BuildMap`
  (bind _terraincubes (`self.TerrainCubes`))
  (bind _terrainboundaries (`self.TerrainBoundaries`))
  (bind (_returnvalue_x _returnvalue_y _returnvalue_z) (`KismetMathLibrary.BreakVector` (`SceneComponent.K2_GetComponentLocation` (`self.DefaultSceneRoot`))))
  (bind _returnvalue (`KismetMathLibrary.FFloor` (/ (`KismetMathLibrary.Conv_IntToDouble` (+ (`self.MapSize`) 2)) 2.0)))
  (bind _returnvalue_2 (- _returnvalue 1))
  (bind _returnvalue_3 (* _returnvalue -1))
  (for _array_element _terrainboundaries
    (`self.K2_DestroyActor` _array_element))
  (`KismetArrayLibrary.Array_Clear` _terrainboundaries)
  (for _array_element_2 _terraincubes
    (`self.K2_DestroyActor` _array_element_2))
  (`KismetArrayLibrary.Array_Clear` _terraincubes)
  (for _index (range _returnvalue_3 (+ _returnvalue_2 1))
    (for _index_2 (range _returnvalue_3 (+ _returnvalue_2 1))
      (if (or (== _index _returnvalue_3) (== _index _returnvalue_2) (== _index_2 _returnvalue_3) (== _index_2 _returnvalue_2))
        (bind _returnvalue_4 (+ _returnvalue_x (`KismetMathLibrary.Conv_IntToDouble` (* _index (`self.TileGap`)))))
        (bind _returnvalue_5 (+ _returnvalue_y (`KismetMathLibrary.Conv_IntToDouble` (* _index_2 (`self.TileGap`)))))
        (bind _returnvalue_6 (`|SpawnActorFromClass` "/Game/Blueprints/BP_Boundaries.BP_Boundaries_C" (`KismetMathLibrary.MakeTransform` (`KismetMathLibrary.MakeVector` _returnvalue_4 _returnvalue_5 (+ _returnvalue_z 110.0))) "Undefined" "OverrideRootScale" null null))
        (`KismetArrayLibrary.Array_Add` (`self.TerrainBoundaries`) _returnvalue_6)
        (else
          (bind _returnvalue_7 (`|SpawnActorFromClass` "/Game/Blueprints/BP_Cube.BP_Cube_C" (`KismetMathLibrary.MakeTransform` (`KismetMathLibrary.MakeVector` _returnvalue_4 _returnvalue_5 _returnvalue_z)) "Undefined" "OverrideRootScale" null null))
          (`KismetArrayLibrary.Array_Add` (`self.TerrainCubes`) _returnvalue_7))))))

(fn `GetMapSize`
  (returns (MaxSize :type Integer))
  (return (* (`self.MapSize`) (`self.TileGap`))))

(fn `GetMinMaxCoordonate`
  (returns (MinPos :type Integer) (MaxPos :type Integer))
  (bind _returnvalue (/ (* (`self.MapSize`) (`self.TileGap`)) 2))
  (return (* _returnvalue -1) _returnvalue))

(fn `UserConstructionScript`)