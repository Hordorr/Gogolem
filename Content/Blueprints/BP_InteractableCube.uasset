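; BP_InteractableCube is a mouse-interactive cube that reacts to hover and click.
; Cursor over and out events report hover to the player's BP_MyChar and scale the cube slightly up, then back to the scale cached in the construction script.
; Clicks notify the same character and print the cube's name.
; BeginPlay creates a dynamic material instance, whose color ChangeColor sets through a vector parameter.
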(event `self.ReceiveBeginPlay`
  (bind _returnvalue (`PrimitiveComponent.CreateDynamicMaterialInstance` (`self.Cube`) 0 null "None"))
  (set `self.MI_Material` _returnvalue))

(event `self.Cube.OnBeginCursorOver`
  (params (TouchedComponent :type "PrimitiveComponent Object Reference"))
  (`/Game/Blueprints/BP_MyChar.UpdateHoverState` (cast `/Game/Blueprints/BP_MyChar` (`Controller.K2_GetPawn` (`GameplayStatics.GetPlayerController` 0)) :!pure true) self true)
  (`SceneComponent.SetWorldScale3D` (`self.Cube`) (* (`self.BaseScale`) (1.05 1.05 1.05))))

(event `self.Cube.OnEndCursorOver`
  (params (TouchedComponent :type "PrimitiveComponent Object Reference"))
  (`/Game/Blueprints/BP_MyChar.UpdateHoverState` (cast `/Game/Blueprints/BP_MyChar` (`Controller.K2_GetPawn` (`GameplayStatics.GetPlayerController` 0)) :!pure true) self false)
  (`SceneComponent.SetWorldScale3D` (`self.Cube`) (`self.BaseScale`)))

(event `self.Cube.OnClicked`
  (params (TouchedComponent :type "PrimitiveComponent Object Reference") (ButtonPressed :type "Key Structure"))
  (`/Game/Blueprints/BP_MyChar.UpdateClickedState` (cast `/Game/Blueprints/BP_MyChar` (`Controller.K2_GetPawn` (`GameplayStatics.GetPlayerController` 0)) :!pure true) self)
  (`KismetSystemLibrary.PrintString` (`KismetStringLibrary.Concat_StrStr` "Clicked : " (`KismetSystemLibrary.GetDisplayName` self)) true true (struct :`G` 0.66 :`B` 1.0 :`A` 1.0) 0.5))

(fn `ChangeColor`
  (params (Color :type "LinearColor Structure (by ref)"))
  (`MaterialInstanceDynamic.SetVectorParameterValue` (`self.MI_Material`) "Color" Color))

(fn `UserConstructionScript`
  (set `self.BaseScale` (`SceneComponent.RelativeScale3D` (`self.Cube`))))