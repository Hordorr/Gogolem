(event `self.ReceiveBeginPlay`
  (`|ExecutionSequence`
    (:`then_0`
      (bind _outactors (`GameplayStatics.GetAllActorsOfClass` "/Game/Blueprints/BP_Cube.BP_Cube_C"))
      (set `self.TerrainCubes` _outactors)
      (`KismetArrayLibrary.Array_AddUnique` (`self.Blocs`) (`self.BaseBloc`))
      (bind _activationstate (`self.UpdateMovementButtons` false))
      (set `self.bButtonActivated` _activationstate)
      (bind _asbp_base_bloc_actor (cast `/Game/Blueprints/BP_BaseBlocActor` (`ChildActorComponent.ChildActor` (`self.BaseBloc`))))
      (`/Game/Blueprints/BP_InteractableCube.ChangeColor` _asbp_base_bloc_actor (`self.Color`) (`/Game/Blueprints/BP_InteractableCube.Cube` _asbp_base_bloc_actor)))
    (:`then_1`
      (bind _returnvalue (`GameplayStatics.GetActorOfClass` "/Game/Blueprints/BP_TerrainGenerator.BP_TerrainGenerator_C"))
      (set `self.TerrainBuilder` _returnvalue))))

(event `Build`
  (params (Cube :type "Actor Object Reference"))
  (bind _previsualisedblocs (`self.PrevisualisedBlocs`))
  (bind _returnvalue (`AddComponent|NODE_AddChildActorComponent-0` :`bManualAttachment` true :`RelativeTransform` (`KismetMathLibrary.MakeTransform` (`self.K2_GetActorLocation` Cube) (struct) (1.0 1.0 0.5))))
  (`KismetSystemLibrary.PrintString` (`KismetSystemLibrary.GetDisplayName` _returnvalue))
  (`SceneComponent.K2_AttachToComponent` _returnvalue (`self.DefaultSceneRoot`) "None" "KeepWorld" "KeepRelative" "KeepRelative" true)
  (`KismetArrayLibrary.Array_AddUnique` (`self.Blocs`) _returnvalue)
  (for _array_element _previsualisedblocs
    (`ActorComponent.K2_DestroyComponent` _array_element))
  (`KismetArrayLibrary.Array_Clear` _previsualisedblocs)
  (set `self.bIsPreviewingblocs` false))

(event `Move`
  (params (PositionToAdd :type "Vector Structure"))
  (bind _returnvalue (+ PositionToAdd (`self.TargetLocation`)))
  (set `self.TargetLocation` (`SceneComponent.K2_GetComponentLocation` (`self.DefaultSceneRoot`)))
  (for _ (range 1 (+ (`self.MovePoint`) 1))
    (bind _canmove (`self.CheckCanMove` _returnvalue))
    (if _canmove
      (set `self.TargetLocation` _returnvalue)))
  (set `self.isMoving` true)
  (bind _activationstate (`self.UpdateMovementButtons` false))
  (set `self.bButtonActivated` _activationstate))

(event `self.ReceiveTick`
  (params (DeltaSeconds :type "Float (single-precision)"))
  (bind _returnvalue (`SceneComponent.K2_GetComponentLocation` (`self.DefaultSceneRoot`)))
  (bind _returnvalue_2 (`KismetMathLibrary.VInterpTo` _returnvalue (`self.TargetLocation`) DeltaSeconds 10.0))
  (`|ExecutionSequence`
    (:`then_0`
      (if (`self.isMoving`)
        (if (not (== _returnvalue _returnvalue_2 :`ErrorTolerance` 0.001))
          (`SceneComponent.K2_SetWorldLocation` (`self.DefaultSceneRoot`) _returnvalue_2 false false)
          (else
            (set `self.isMoving` false)))))))

(fn `CheckCanMove`
  (params (TargetPos :type "Vector Structure"))
  (returns (CanMove :type Boolean))
  (bind _validmove (`self.Move PossibleInMap` TargetPos))
  (bind _validmove_2 (`self.MovePossibleObstruction` TargetPos))
  (return (and _validmove _validmove_2)))

(fn `Get Possible Place for Bloc`
  (returns (AvalaibleSpaces :type "Array of Vector Structure"))
  (locals (AvailableSpaces :type "Array of Vector Structure") (AvalaibleSpace2 :type "Array of Vector Structure"))
  (bind _availablespaces (`local.AvailableSpaces`))
  (`KismetArrayLibrary.Array_Clear` (`local.AvailableSpaces`))
  (for _array_element (`self.Blocs`)
    (`|ExecutionSequence`
      (:`then_0`
        (bind (_relativelocation_x _relativelocation_y _relativelocation_z) (`KismetMathLibrary.BreakVector` (`SceneComponent.RelativeLocation` _array_element)))
        (bind _returnvalue (`KismetMathLibrary.MakeVector` (`KismetMathLibrary.Conv_IntToDouble` (`KismetMathLibrary.Round` _relativelocation_x)) (`KismetMathLibrary.Conv_IntToDouble` (`KismetMathLibrary.Round` _relativelocation_y)) (`KismetMathLibrary.Conv_IntToDouble` (`KismetMathLibrary.Round` _relativelocation_z))))
        (`KismetArrayLibrary.Array_AddUnique` _availablespaces (+ _returnvalue (110.0 0.0 0.0))))
      (:`then_1`
        (`KismetArrayLibrary.Array_AddUnique` _availablespaces (+ _returnvalue (-110.0 0.0 0.0))))
      (:`then_2`
        (`KismetArrayLibrary.Array_AddUnique` _availablespaces (+ _returnvalue (0.0 110.0 0.0))))
      (:`then_3`
        (`KismetArrayLibrary.Array_AddUnique` _availablespaces (+ _returnvalue (0.0 -110.0 0.0))))))
  (for _array_element_2 (`self.Blocs`)
    (for (_array_element_3 _array_index) (`local.AvailableSpaces`)
      (if (== _array_element_3 (`SceneComponent.RelativeLocation` _array_element_2) :`ErrorTolerance` 10.0)
        (`KismetArrayLibrary.Array_Remove` (`local.AvailableSpaces`) _array_index))))
  (return (`local.AvailableSpaces`)))

(fn `Get Used Xand Y`
  (returns (XList :type "Array of Integer") (YList :type "Array of Integer"))
  (locals (Xs :type "Array of Integer") (Ys :type "Array of Integer"))
  (`KismetArrayLibrary.Array_Clear` (`local.Xs`))
  (`KismetArrayLibrary.Array_Clear` (`local.Ys`))
  (for _array_element (`self.Blocs`)
    (`|ExecutionSequence`
      (:`then_0`
        (bind (_returnvalue_x _returnvalue_y) (`KismetMathLibrary.BreakVector` (`SceneComponent.K2_GetComponentLocation` _array_element)))
        (`KismetArrayLibrary.Array_AddUnique` (`local.Xs`) (`KismetMathLibrary.Conv_Int64ToInt` (`KismetMathLibrary.Round64` _returnvalue_x))))
      (:`then_1`
        (`KismetArrayLibrary.Array_AddUnique` (`local.Ys`) (`KismetMathLibrary.Conv_Int64ToInt` (`KismetMathLibrary.Round64` _returnvalue_y))))))
  (return (`local.Xs`) (`local.Ys`)))

(fn `Move Cubes`
  (params (deltaSeconds :type "Float (double-precision)") (Target :type "Vector Structure")))

(fn `Move PossibleInMap`
  (params (TargetPos :type "Vector Structure"))
  (returns (ValidMove :type Boolean))
  (locals (bCanMove :type Boolean :default false))
  (bind (_minpos _maxpos) (`/Game/Blueprints/BP_TerrainGenerator.GetMinMaxCoordonate` (`self.TerrainBuilder`)))
  (for _array_element (`self.Blocs`)
    (bind (_returnvalue_x _returnvalue_y) (`KismetMathLibrary.BreakVector` (+ TargetPos (`SceneComponent.RelativeLocation` _array_element))))
    (bind _output_get (set `local.bCanMove` (and (>= (`KismetMathLibrary.Round` _returnvalue_x) _minpos) (<= (`KismetMathLibrary.Round` _returnvalue_x) _maxpos) (>= (`KismetMathLibrary.Round` _returnvalue_y) _minpos) (<= (`KismetMathLibrary.Round` _returnvalue_y) _maxpos))))
    (if (not _output_get)
      (break)))
  (return (`local.bCanMove`)))

(fn `MovePossibleObstruction`
  (params (TargetPos :type "Vector Structure"))
  (returns (ValidMove :type Boolean))
  (locals (bCanMove :type Boolean :default true) (BlockingElements :type "Array of Actor Object Reference") (bCollision :type Boolean))
  (bind _outactors (`GameplayStatics.GetAllActorsOfClassWithTag` "/Game/Blueprints/BP_BaseBlocActor.BP_BaseBlocActor_C" "ObstructingElement"))
  (set `local.BlockingElements` _outactors)
  (for _array_element (`self.Blocs`)
    (`KismetArrayLibrary.Array_RemoveItem` (`local.BlockingElements`) (`ChildActorComponent.ChildActor` _array_element)))
  (for _array_element_2 (`self.Blocs`)
    (for _array_element_3 (`local.BlockingElements`)
      (bind _output_get (set `local.bCollision` (== (`self.K2_GetActorLocation` _array_element_3) (+ (`SceneComponent.RelativeLocation` _array_element_2) TargetPos) :`ErrorTolerance` 0.1)))
      (if _output_get
        (`KismetSystemLibrary.PrintString` "Collsion")
        (`KismetSystemLibrary.DrawDebugSphere` (`self.K2_GetActorLocation` _array_element_3) 100.0 12 (struct :`R` 1.0 :`G` 1.0 :`B` 1.0 :`A` 1.0) 1.0)
        (if (`local.bCanMove`)
          (set `local.bCanMove` false))
        (else
          (`KismetSystemLibrary.PrintString` "No Colision")))))
  (return (`local.bCanMove`)))

(fn `SpawnBlocAtLocation`
  (params (A :type "Vector Structure"))
  (returns (ReturnValue :type "ChildActorComponent Object Reference"))
  (bind _returnvalue (`AddComponent|NODE_AddChildActorComponent-1` :`RelativeTransform` (`KismetMathLibrary.MakeTransform` A)))
  (return _returnvalue))

(fn `Update Possible Attack Pos`
  (locals (Xs :type "Array of Integer") (Ys :type "Array of Integer"))
  (for _ (`self.Blocs`)
    (`KismetSystemLibrary.PrintString` "Hello")
    (bind (_xlist _ylist) (`self.Get Used Xand Y`))
    (for _array_element (`self.TerrainCubes`)
      (bind _returnvalue (`SceneComponent.K2_GetComponentLocation` (`/Game/Blueprints/BP_InteractableCube.Cube` _array_element)))
      (if (or (`KismetArrayLibrary.Array_Contains` _xlist (`KismetMathLibrary.Round` (.x _returnvalue))) (`KismetArrayLibrary.Array_Contains` _ylist (`KismetMathLibrary.Round` (.y _returnvalue))))
        (`KismetSystemLibrary.DrawDebugSphere` _returnvalue 75.0 12 (struct :`R` 1.0 :`G` 1.0 :`B` 1.0 :`A` 1.0) 2.0))))
  (return))

(fn `Update Possible Build Pos`
  (params (bool :type Boolean))
  (locals (PreviewBloc :type "Array of ChildActorComponent Object Reference"))
  (bind _previsualisedblocs (`self.PrevisualisedBlocs`))
  (if bool
    (`KismetSystemLibrary.PrintString` "Hello")
    (for _array_element _previsualisedblocs
      (`ActorComponent.K2_DestroyComponent` _array_element))
    (`KismetArrayLibrary.Array_Clear` _previsualisedblocs)
    (set `self.bIsPreviewingblocs` false)
    (return)
    (else
      (`KismetSystemLibrary.PrintString` "dgdh")
      (bind _avalaiblespaces (`self.Get Possible Place for Bloc`))
      (for _array_element_2 _avalaiblespaces
        (bind _returnvalue (`self.SpawnBlocAtLocation` _array_element_2))
        (`KismetArrayLibrary.Array_AddUnique` (`self.PrevisualisedBlocs`) _returnvalue))
      (set `self.bIsPreviewingblocs` true)
      (return))))

(fn `UpdateMovementButtons`
  (params (bIsActive :type Boolean))
  (returns (ActivationState :type Boolean))
  (bind _cube (`/Game/Blueprints/BP_InteractableCube.Cube` (cast `/Game/Blueprints/BP_MovementButton` (`ChildActorComponent.ChildActor` (`self.Down`)) :!pure true)))
  (set `self.bButtonActivated` bIsActive)
  (`SceneComponent.SetVisibility` _cube bIsActive false)
  (`SceneComponent.SetVisibility` (`/Game/Blueprints/BP_InteractableCube.Cube` (cast `/Game/Blueprints/BP_MovementButton` (`ChildActorComponent.ChildActor` (`self.Left`)) :!pure true)) bIsActive false)
  (`SceneComponent.SetVisibility` (`/Game/Blueprints/BP_InteractableCube.Cube` (cast `/Game/Blueprints/BP_MovementButton` (`ChildActorComponent.ChildActor` (`self.Right`)) :!pure true)) bIsActive false)
  (`SceneComponent.SetVisibility` (`/Game/Blueprints/BP_InteractableCube.Cube` (cast `/Game/Blueprints/BP_MovementButton` (`ChildActorComponent.ChildActor` (`self.Top`)) :!pure true)) bIsActive false)
  (if bIsActive
    (`PrimitiveComponent.SetCollisionEnabled` _cube "QueryAndPhysics")
    (`PrimitiveComponent.SetCollisionEnabled` (`/Game/Blueprints/BP_InteractableCube.Cube` (cast `/Game/Blueprints/BP_MovementButton` (`ChildActorComponent.ChildActor` (`self.Left`)) :!pure true)) "QueryAndPhysics")
    (`PrimitiveComponent.SetCollisionEnabled` (`/Game/Blueprints/BP_InteractableCube.Cube` (cast `/Game/Blueprints/BP_MovementButton` (`ChildActorComponent.ChildActor` (`self.Right`)) :!pure true)) "QueryAndPhysics")
    (`PrimitiveComponent.SetCollisionEnabled` (`/Game/Blueprints/BP_InteractableCube.Cube` (cast `/Game/Blueprints/BP_MovementButton` (`ChildActorComponent.ChildActor` (`self.Top`)) :!pure true)) "QueryAndPhysics")
    (else
      (`PrimitiveComponent.SetCollisionEnabled` (`/Game/Blueprints/BP_InteractableCube.Cube` (cast `/Game/Blueprints/BP_MovementButton` (`ChildActorComponent.ChildActor` (`self.Top`)) :!pure true)) "NoCollision")
      (`PrimitiveComponent.SetCollisionEnabled` (`/Game/Blueprints/BP_InteractableCube.Cube` (cast `/Game/Blueprints/BP_MovementButton` (`ChildActorComponent.ChildActor` (`self.Right`)) :!pure true)) "NoCollision")
      (`PrimitiveComponent.SetCollisionEnabled` (`/Game/Blueprints/BP_InteractableCube.Cube` (cast `/Game/Blueprints/BP_MovementButton` (`ChildActorComponent.ChildActor` (`self.Left`)) :!pure true)) "NoCollision")
      (`PrimitiveComponent.SetCollisionEnabled` _cube "NoCollision")))
  (return bIsActive))

(fn `UserConstructionScript`)