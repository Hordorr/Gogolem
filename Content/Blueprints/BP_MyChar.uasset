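; Player character for a grid-based, turn-based pawn game that turns input into pawn selection, movement, building, attack previews, tile painting and turn changes.
; BeginPlay caches every BP_Cube with its XY position and binds cube hover and click events.
; CheckClickTarget casts clicked objects to route pawn selection, movement or build buttons, with actions gated by the selected pawn's state.
; PaintBlocUnder matches the pawn's child-actor positions to cached cubes to paint them by team.
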(event `InputAction|FirstMouseInput`
  (params (Key :type "Key Structure"))
  ;[1 1 1] ClickGaucheInput
  (:`Pressed`
    (`/Engine/EditorBlueprintResources/StandardMacros.DoOnce` false :!label _label
      (:`Completed`
        (`|ExecutionSequence`
          (:`then_0`
            (if (`KismetSystemLibrary.IsValid` (`self.SelectedPawn`))
              _))))))
  (:`Released`
    (goto _label :!via `Reset`)))

(event `self.ReceiveTick`
  (params (DeltaSeconds :type "Float (single-precision)"))
  (bind (_bblockinghit _binitialoverlap _time _distance _location _impactpoint _normal _impactnormal _physmat _hitactor _hitcomponent) (`GameplayStatics.BreakHitResult` (`PlayerController.GetHitResultUnderCursorByChannel` (`GameplayStatics.GetPlayerController` 0) "TraceTypeQuery4" true)))
  (`|ExecutionSequence`
    (:`then_0`
      (if _bblockinghit
        (bind _asbp_pawn_base (cast `/Game/Blueprints/BP_PawnBase` (`self.GetParentActor` (`ActorComponent.GetOwner` _hitcomponent)))
          (:`then`
            (bind _output_get (set `self.HoveredPawn` _asbp_pawn_base))
            (set `self.OldHoveredPawn` _output_get))
          (:`CastFailed`
            (set `self.HoveredPawn` null :!label _label_2)))
        (else
          (goto _label_2))))
    (:`then_1`
      (`KismetSystemLibrary.PrintString` (`KismetSystemLibrary.GetDisplayName` (`self.SelectedPawn`)) true false (struct :`G` 0.66 :`B` 1.0 :`A` 1.0) (`GameplayStatics.GetWorldDeltaSeconds`)))))

(event `InputAction|SecondMouseinput`
  (params (Key :type "Key Structure"))
  ;[1 1 1] ClickDroitInput
  (:`Pressed`
    (`/Engine/EditorBlueprintResources/StandardMacros.DoOnce` false :!label _label_3
      (:`Completed`
        (set `self.SelectedPawn` null))))
  (:`Released`
    (goto _label_3 :!via `Reset`)))

(event `InputAction|PaintBlocInput`
  (params (Key :type "Key Structure"))
  ;[1 1 1] Paint
  (:`Pressed`
    (`/Engine/EditorBlueprintResources/StandardMacros.DoOnce` false :!label _label_4
      (:`Completed`
        (for _array_element (`self.GetAllChildActors` (`self.SelectedPawn`) true)
          (`KismetSystemLibrary.PrintString` (`KismetSystemLibrary.GetDisplayName` _array_element))
          (for _array_element_2 (`self.Cubes`)
            (bind (_actor _position) (break `/Game/Blueprints/S_Cube` _array_element_2))
            (bind (_returnvalue_x _returnvalue_y) (`KismetMathLibrary.BreakVector` (`self.K2_GetActorLocation` _array_element)))
            (if (== _position (`KismetMathLibrary.MakeVector2D` _returnvalue_x _returnvalue_y))
              (`/Game/Blueprints/BP_Cube.Paint` _actor (`self.Team`))))))))
  (:`Released`
    (goto _label_4 :!via `Reset`)))

(event `InputAction|AttackInput`
  (params (Key :type "Key Structure"))
  (bind _selectedpawn (`self.SelectedPawn`))
  (:`Pressed`
    (`/Engine/EditorBlueprintResources/StandardMacros.DoOnce` false :!label _label_5
      (:`Completed`
        (`/Engine/EditorBlueprintResources/StandardMacros.IsValid` _selectedpawn
          (:`Is Valid`
            (`/Game/Blueprints/BP_PawnBase.Update Possible Attack Pos` _selectedpawn))))))
  (:`Released`
    (goto _label_5 :!via `Reset`)))

(event `self.ReceiveBeginPlay`
  (`|ExecutionSequence`
    (:`then_0`
      (set `self.SelectedPawn` null))
    (:`then_1`
      (bind _outactors (`GameplayStatics.GetAllActorsOfClass` "/Game/Blueprints/BP_Cube.BP_Cube_C"))
      (for _array_element _outactors
        (bind (_returnvalue_x _returnvalue_y) (`KismetMathLibrary.BreakVector` (`self.K2_GetActorLocation` _array_element)))
        (`KismetArrayLibrary.Array_AddUnique` (`self.Cubes`) (make `/Game/Blueprints/S_Cube` _array_element (`KismetMathLibrary.MakeVector2D` _returnvalue_x _returnvalue_y)))))
    (:`then_2`
      (add `self.UpdateHoverState` (delegate `CursorHoverCube`)))
    (:`then_3`
      (add `self.UpdateClickedState` (delegate `ClickedCube`)))))

(event `CursorHoverCube`
  (params (Cube :type "Actor Object Reference") (bIsHovered :type Boolean))
  (`/Engine/EditorBlueprintResources/StandardMacros.IsValid` Cube
    (:`Is Valid`
      (set `self.HoveredMap` Cube))))

(event `ClickedCube`
  (params (Cube :type "Actor Object Reference"))
  (`self.CheckClickTarget` Cube))

(event `PawnClicked`
  (params (Pawn :type "/Game/Blueprints/BP_PawnBase Object Reference"))
  ;[1 0.7163 0] IfClickedOnPawn
  (if (!= Pawn (`self.SelectedPawn`))
    (set `/Game/Blueprints/BP_PawnBase.State` "NewEnumerator2" (`self.SelectedPawn`))
    (bind _output_get (set `self.SelectedPawn` Pawn))
    (set `/Game/Blueprints/BP_PawnBase.State` "NewEnumerator5" _output_get)))

(event `MoveButtonClicked`
  (params (MoveButton :type "/Game/Blueprints/BP_MovementButton Object Reference"))
  (if (`|EnumEquality` (`/Game/Blueprints/BP_PawnBase.State` (`self.SelectedPawn`)) "NewEnumerator0")
    (`/Game/Blueprints/BP_PawnBase.Move` (`self.SelectedPawn`) (`/Game/Blueprints/BP_MovementButton.PositionToAdd` MoveButton) (`/Game/Blueprints/BP_MovementButton.Direction` MoveButton))))

(event `InputAction|TstInput`
  (params (Key :type "Key Structure"))
  (:`Pressed`
    (`/Engine/EditorBlueprintResources/StandardMacros.DoOnce` false :!label _label_6
      (:`Completed`
        (`self.GoToBuildMod`))))
  (:`Released`
    (goto _label_6 :!via `Reset`)))

(event `BuildButtonClicked`
  (params (BuildButton :type "/Game/Blueprints/BP_TranslusentBloc Object Reference"))
  (if (`|EnumEquality` (`/Game/Blueprints/BP_PawnBase.State` (`self.SelectedPawn`)) "NewEnumerator1")
    (`/Game/Blueprints/BP_PawnBase.Build` (`self.SelectedPawn`) BuildButton)
    (`/Game/Blueprints/BP_PawnBase.UpdateState` (`self.SelectedPawn`) "NewEnumerator5")))

(event `Key|V`
  (params (Key :type "Key Structure"))
  (:`Pressed`
    (`/Engine/EditorBlueprintResources/StandardMacros.DoOnce` false :!label _label_7
      (:`Completed`
        (`self.GoToMoveMod`))))
  (:`Released`
    (goto _label_7 :!via `Reset`)))

(event `InputAction|ChangeTurnInput`
  (params (Key :type "Key Structure"))
  (:`Pressed`
    (`/Engine/EditorBlueprintResources/StandardMacros.DoOnce` false :!label _label_8
      (:`Completed`
        (`/Game/Blueprints/BP_MyPlayerController.ChangePlayer` (cast `/Game/Blueprints/BP_MyPlayerController` (`GameplayStatics.GetPlayerController` 0) :!pure true)))))
  (:`Released`
    (goto _label_8 :!via `Reset`)))

(event `GoToBuildMod`
  (bind _selectedpawn (`self.SelectedPawn`))
  (if (`|EnumEquality` (`/Game/Blueprints/BP_PawnBase.State` (`self.SelectedPawn`)) "NewEnumerator6")
    _
    (elif (`|EnumEquality` (`/Game/Blueprints/BP_PawnBase.State` (`self.SelectedPawn`)) "NewEnumerator1")
      (`/Game/Blueprints/BP_PawnBase.UpdateState` _selectedpawn "NewEnumerator2")
      (else
        (`/Game/Blueprints/BP_PawnBase.UpdateState` _selectedpawn "NewEnumerator1")))))

(event `GoToMoveMod`
  (if (`|EnumEquality` (`/Game/Blueprints/BP_PawnBase.State` (`self.SelectedPawn`)) "NewEnumerator6")
    (`KismetSystemLibrary.PrintString` "locked")
    (elif (`|EnumEquality` (`/Game/Blueprints/BP_PawnBase.State` (`self.SelectedPawn`)) "NewEnumerator0")
      (`/Game/Blueprints/BP_PawnBase.UpdateState` (`self.SelectedPawn`) "NewEnumerator2")
      (else
        (`/Game/Blueprints/BP_PawnBase.UpdateState` (`self.SelectedPawn`) "NewEnumerator0")))))

(fn `CheckClickTarget`
  (params (ObjectClicked :type "Actor Object Reference"))
  (`/Engine/EditorBlueprintResources/StandardMacros.IsValid` (`self.SelectedPawn`)
    (:`Is Valid`
      (bind _asbp_translusent_bloc (cast `/Game/Blueprints/BP_TranslusentBloc` ObjectClicked)
        (:`then`
          (`self.BuildButtonClicked` _asbp_translusent_bloc))
        (:`CastFailed`
          (bind _asbp_base_bloc_actor (cast `/Game/Blueprints/BP_BaseBlocActor` ObjectClicked)
            (:`then`
              (bind _asbp_pawn_base (cast `/Game/Blueprints/BP_PawnBase` (`self.GetParentActor` _asbp_base_bloc_actor)))
              (`self.PawnClicked` _asbp_pawn_base))
            (:`CastFailed`
              (bind _asbp_movement_button (cast `/Game/Blueprints/BP_MovementButton` ObjectClicked))
              (`self.MoveButtonClicked` _asbp_movement_button))))))
    (:`Is Not Valid`
      (bind _asbp_pawn_base_2 (cast `/Game/Blueprints/BP_PawnBase` (`self.GetParentActor` ObjectClicked)))
      (set `self.SelectedPawn` _asbp_pawn_base_2))))

(fn `UserConstructionScript`)