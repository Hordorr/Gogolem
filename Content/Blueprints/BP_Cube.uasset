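; BP_Cube is a cube that players can paint in their own color.
; ChangeState handles the Painted state by passing P1Color or P2Color to ChangeColor according to the player index, then storing the state in PaintState.
; The Paint event is empty, and disconnected nodes hold color-index logic that sets a green material for color 1 and does nothing for color 2.
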(event `Paint`
  (params (Color :type Integer)))

(fn `ChangeState`
  (params (NewState :type "/Game/Blueprints/E_BaseCubeState Enum" :default "NewEnumerator1") (PlayerIndex :type Integer))
  (switch `/Game/Blueprints/E_BaseCubeState` NewState
    (:`NewEnumerator0`
      (switch `int` PlayerIndex
        (:`1`
          (`self.ChangeColor` (`self.P1Color`)))
        (:`2`
          (`self.ChangeColor` (`self.P2Color`))))
      (set `self.PaintState` NewState))))

(fn `UserConstructionScript`)