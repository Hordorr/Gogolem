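; Player controller Blueprint that tracks whose turn it is in a two-player, turn-based setup.
; The EndTurn event calls ChangePlayer, which switches PlayerIndex to 2 when it is 1 and to 1 otherwise.
; Tick prints the current player index on screen every frame as a debug readout, using DeltaSeconds as the display duration.
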(event `self.ReceiveTick`
  (params (DeltaSeconds :type "Float (single-precision)"))
  (`KismetSystemLibrary.PrintString` (`KismetStringLibrary.Concat_StrStr` "Player: " (`KismetStringLibrary.Conv_IntToString` (`self.PlayerIndex`))) true true (struct :`G` 0.66 :`B` 1.0 :`A` 1.0) DeltaSeconds))

(event `EndTurn`
  (`self.ChangePlayer`))

(fn `ChangePlayer`
  (if (== (`self.PlayerIndex`) 1)
    (set `self.PlayerIndex` 2)
    (else
      (set `self.PlayerIndex` 1))))

(fn `UserConstructionScript`)